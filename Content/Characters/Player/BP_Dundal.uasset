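; BP_Dundal is a player character Blueprint with Enhanced Input movement, a primary attack and five ability slots.
; BeginPlay adds the IMC_Dundal mapping context and caches a BP_SectorEnforcer reference, unused in these graphs.
; Inputs forward to AbilityComponent slots or PrimaryAttackComponent with debug prints; R and Interrupt inputs trigger slots opposite to their messages.
; The BP_DontFlinch assignment to Engage is disconnected and never runs.
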(event Input|EnhancedActionEvents|EnhancedInputActionIA_AbilityQ
  (params (ActionValue :type Boolean) (ElapsedSeconds :type Float%20%28double-precision%29) (TriggeredSeconds :type Float%20%28double-precision%29) (InputAction :type Input%20Action%20Object%20Reference :default "/Game/Characters/Player/Input/IA_AbilityQ.IA_AbilityQ"))
  (:Started
    (Class|AbilityComponent|ExecuteSlot (Variables|Default|GetAbilityComponent) "Engage")
    (Development|PrintString "Q Pressed, using Engage Ability!")))

(event Input|EnhancedActionEvents|EnhancedInputActionIA_AbilityW
  (params (ActionValue :type Boolean) (ElapsedSeconds :type Float%20%28double-precision%29) (TriggeredSeconds :type Float%20%28double-precision%29) (InputAction :type Input%20Action%20Object%20Reference :default "/Game/Characters/Player/Input/IA_AbilityW.IA_AbilityW"))
  (:Started
    (Class|AbilityComponent|ExecuteSlot (Variables|Default|GetAbilityComponent) "Follow")
    (Development|PrintString "W Pressed, using Follow-up Ability!")))

(event Input|EnhancedActionEvents|EnhancedInputActionIA_AbilityE
  (params (ActionValue :type Boolean) (ElapsedSeconds :type Float%20%28double-precision%29) (TriggeredSeconds :type Float%20%28double-precision%29) (InputAction :type Input%20Action%20Object%20Reference :default "/Game/Characters/Player/Input/IA_AbilityE.IA_AbilityE"))
  (:Started
    (Class|AbilityComponent|ExecuteSlot (Variables|Default|GetAbilityComponent) "Counter")
    (Development|PrintString "E Pressed, using Counter Ability!")))

(event Input|EnhancedActionEvents|EnhancedInputActionIA_AbilityR
  (params (ActionValue :type Boolean) (ElapsedSeconds :type Float%20%28double-precision%29) (TriggeredSeconds :type Float%20%28double-precision%29) (InputAction :type Input%20Action%20Object%20Reference :default "/Game/Characters/Player/Input/IA_AbilityR.IA_AbilityR"))
  (:Started
    (Class|AbilityComponent|ExecuteSlot (Variables|Default|GetAbilityComponent) "Interrupt")
    (Development|PrintString "R Pressed, using Ultimate Ability!")))

(event Input|EnhancedActionEvents|EnhancedInputActionIA_AbilityInterrupt
  (params (ActionValue :type Boolean) (ElapsedSeconds :type Float%20%28double-precision%29) (TriggeredSeconds :type Float%20%28double-precision%29) (InputAction :type Input%20Action%20Object%20Reference :default "/Game/Characters/Player/Input/IA_AbilityInterrupt.IA_AbilityInterrupt"))
  (:Started
    (Class|AbilityComponent|ExecuteSlot (Variables|Default|GetAbilityComponent) "Ultimate")
    (Development|PrintString "T Pressed, Interrupting Enemy!")))

(event Input|EnhancedActionEvents|EnhancedInputActionIA_PrimaryAttack
  (params (ActionValue :type Boolean) (ElapsedSeconds :type Float%20%28double-precision%29) (TriggeredSeconds :type Float%20%28double-precision%29) (InputAction :type Input%20Action%20Object%20Reference :default "/Game/Characters/Player/Input/IA_PrimaryAttack.IA_PrimaryAttack"))
  (:Started
    (Class|PrimaryAttackComponent|PerformAttack (Variables|Default|GetPrimaryAttackComponent))
    (Development|PrintString "Attack performed")))

(event Input|EnhancedActionEvents|EnhancedInputActionIA_Move
  (params (ActionValue :type Vector%202D%20Structure) (ElapsedSeconds :type Float%20%28double-precision%29) (TriggeredSeconds :type Float%20%28double-precision%29) (InputAction :type Input%20Action%20Object%20Reference :default "/Game/Characters/Player/Input/IA_Move.IA_Move"))
  (bind (_x _y) (Math|Vector2D|BreakVector2D ActionValue))
  (Pawn|Input|AddMovementInput (Math|Vector|GetRightVector (Pawn|GetControlRotation :!class /Script/Engine.Pawn)) _x false)
  (Pawn|Input|AddMovementInput (Math|Vector|GetForwardVector (Pawn|GetControlRotation :!class /Script/Engine.Pawn)) _y false))

(event EventBeginPlay
  (Input|AddMappingContext (PlayerController|LocalPlayerSubsystems|GetEnhancedInputLocalPlayerSubsystem (Game|GetPlayerController 0)) "/Game/Characters/Player/Input/IMC_Dundal.IMC_Dundal" 0 "(bIgnoreAllPressedKeysUntilRelease=True,bForceImmediately=False,bNotifyUserSettings=False)")
  (bind _returnvalue (Actor|GetActorOfClass "/Game/Characters/Enemies/BP_SectorEnforcer.BP_SectorEnforcer_C"))
  (Variables|Default|SetSectorEnforcerRef _returnvalue))

(fn ConstructionScript)
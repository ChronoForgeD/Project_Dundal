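; BP_DontFlinch is a player ability, apparently used by Dundal, that deals direct damage to a fighter target.
; ExecuteAbility calls the parent implementation, then casts the target to FighterCharacterBase and applies the AbilityData damage through its HealthComponent.
; Debug prints report the ability name and damage, or a failed cast that deals no damage.
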(event EventExecuteAbility
  (params (Instigator :type Actor%20Object%20Reference) (Target :type Actor%20Object%20Reference))
  (bind _self self)
  (bind _abilitydata (Variables|Default|GetAbilityData _self))
  (|CallParentFunction Instigator Target)
  (bind _asfighter_character_base (Utilities|Casting|CastToFighterCharacterBase Target)
    (:then
      (Class|HealthComponent|TakeDamage (Variables|/Script/Project_Dundal.FighterCharacterBase|GetHealthComponent _asfighter_character_base) (.damage _abilitydata))
      (Development|PrintString 0 (Utilities|String|Append "Dundal Used: " (Utilities|String|ToString(Text) (.abilityname _abilitydata)) " It Dealt: " (Utilities|String|ToString(Float) (.damage _abilitydata)))))
    (:CastFailed
      (Development|PrintString 0 "Cast Failed will not deal damage"))))